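; BP_EnemyBase is the base enemy Blueprint that takes damage and dies when its health runs out.
; On AnyDamage it subtracts the damage from its HealthComponent's Health and prints the remaining value as a Spanish debug message.
; When Health reaches zero or below, the actor destroys itself; the construction script is empty.
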(event `self.ReceiveAnyDamage`
  (params (Damage :type "Float (single-precision)") (DamageType :type "DamageType Object Reference") (InstigatedBy :type "Controller Object Reference") (DamageCauser :type "Actor Object Reference"))
  (bind _healthcomponent (`self.HealthComponent`))
  (bind _health (`HealthComponent.Health` _healthcomponent))
  (set `HealthComponent.Health` (- _health Damage) _healthcomponent)
  (`KismetSystemLibrary.PrintString` (`KismetStringLibrary.Concat_StrStr` "la vida actual es" (`KismetStringLibrary.Conv_DoubleToString` _health)))
  (if (<= (`HealthComponent.Health` (`self.HealthComponent`)) 0.0)
    (`self.K2_DestroyActor`)))

(fn `UserConstructionScript`)