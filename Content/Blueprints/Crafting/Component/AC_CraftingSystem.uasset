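; Actor component that runs the crafting system, deciding which recipes are unlocked and toggling the crafting menu.
; On begin play it creates the crafting widget; the crafting input shows or hides it, switching input mode, cursor and game pause.
; Initialization reads the recipe data table, async-loads unloaded item classes, unlocks rows meeting the level requirement, and prints them.
; The unlocked list populates the widget's slots when opened.
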(event `self.ReceiveBeginPlay`
  (bind _returnvalue (`|CreateWidget` "/Game/Blueprints/Crafting/Widget/W_Crafting.W_Crafting_C"))
  (set `self.Crafting Ref` _returnvalue))

(event `EnhancedInput|/Game/Input/Actions/IA_Crafting`
  (params (ActionValue :type Boolean) (ElapsedSeconds :type "Float (double-precision)") (TriggeredSeconds :type "Float (double-precision)") (InputAction :type "InputAction Object Reference" :default "/Game/Input/Actions/IA_Crafting.IA_Crafting"))
  (bind _returnvalue (`GameplayStatics.GetPlayerController` 0))
  (bind _returnvalue_2 (`GameplayStatics.GetPlayerController` 0))
  (bind _crafting_ref (`self.Crafting Ref`))
  (bind _crafting_ref_2 (`self.Crafting Ref`))
  (bind _crafting_ref_3 (`self.Crafting Ref`))
  (:`Started`
    (if (`Widget.IsVisible` _crafting_ref_2)
      (`Widget.RemoveFromParent` _crafting_ref_2)
      (set `PlayerController.bShowMouseCursor` false _returnvalue)
      (`WidgetBlueprintLibrary.SetInputMode_GameOnly` _returnvalue)
      (`GameplayStatics.SetGamePaused` false)
      (else
        (`WidgetBlueprintLibrary.SetInputMode_GameAndUIEx` _returnvalue_2 _crafting_ref_3)
        (set `PlayerController.bShowMouseCursor` true _returnvalue_2)
        (`UserWidget.AddToViewport` _crafting_ref_3 0)
        (`/Game/Blueprints/Crafting/Widget/W_Crafting.UpdateCraftingSlots` (`self.Crafting Ref`) "/Game/Blueprints/Crafting/Datas/DT_Crafting.DT_Crafting" (`self.UnlockedCratgableItem`) "NewEnumerator0")
        (`GameplayStatics.SetGamePaused` true)
        (`Widget.SetVisibility` _crafting_ref "Visible")
        (`/Game/Blueprints/Crafting/Widget/W_Crafting.HideIngredients` _crafting_ref)))))

(event `InitCraftingCalculate`
  (params (DataCrafting :type "DataTable Object Reference"))
  (set `self.Data Crafting` DataCrafting)
  (bind _outrownames (`DataTableFunctionLibrary.GetDataTableRowNames` (`self.Data Crafting`)))
  (set `self.AllItemsCraftables` _outrownames)
  (`self.CalculateItemsCrafteables`)
  (`self.PrintUnlockedItems`))

(event `LoadAsync`
  (params (ItemBase :type "/Game/Blueprints/Crafting/Objetos/BP_BasePickupItem Soft Class Reference"))
  (`|LoadAssetClass` ItemBase))

(fn `CalculateItemsCrafteables`
  (locals (LocalItemsCraftables :type Name) (CurrentItemRow :type "/Game/Blueprints/Crafting/Datas/S_Crafting Structure"))
  (for _array_element (`self.AllItemsCraftables`)
    (set `local.LocalItemsCraftables` _array_element)
    (if (not (`KismetArrayLibrary.Array_Contains` (`self.UnlockedCratgableItem`) (`local.LocalItemsCraftables`)))
      (bind _out_row (`self.GetCraftableItemFromName` (`local.LocalItemsCraftables`)))
      (set `local.CurrentItemRow` _out_row)
      (if (not (`KismetSystemLibrary.IsValidClass` (`|ConvertAsset` (`.ItemBase_19_C01A5FBC4117070BA4FDE9BF11B06D2D` (break `/Game/Blueprints/Crafting/Datas/S_Crafting` (`local.CurrentItemRow`))))))
        (`self.LoadAsync` (`.ItemBase_19_C01A5FBC4117070BA4FDE9BF11B06D2D` (break `/Game/Blueprints/Crafting/Datas/S_Crafting` (`local.CurrentItemRow`)))))
      (if (== (`.RequierdLvl_11_04472C984BC80AFE728130AB3A2DB66D` (break `/Game/Blueprints/Crafting/Datas/S_Crafting` (`local.CurrentItemRow`))) 0)
        (`KismetArrayLibrary.Array_Add` (`self.UnlockedCratgableItem`) (`local.LocalItemsCraftables`) :!label _label)
        (elif (>= (`self.CurrentLvl`) (`.RequierdLvl_11_04472C984BC80AFE728130AB3A2DB66D` (break `/Game/Blueprints/Crafting/Datas/S_Crafting` (`local.CurrentItemRow`))))
          (goto _label))))))

(fn `GetCraftableItemFromName`
  (params (RowName :type Name))
  (returns (`Out Row` :type "/Game/Blueprints/Crafting/Datas/S_Crafting Structure"))
  (`DataTableFunctionLibrary.DoesDataTableRowExist` (`self.Data Crafting`) RowName)
  (if true
    (bind _returnvalue (`|GetDataTableRow` (`self.Data Crafting`) RowName)
      (:`then`
        (return _returnvalue)))))

(fn `PrintUnlockedItems`
  (for _array_element (`self.UnlockedCratgableItem`)
    (`KismetSystemLibrary.PrintString` (`KismetStringLibrary.Conv_NameToString` _array_element))))