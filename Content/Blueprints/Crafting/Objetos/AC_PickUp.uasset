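; Player inventory component that handles item pickup and the inventory side of crafting.
; On take-item input, a camera-forward sphere trace finds a BP_BasePickupItem, stores its data in a name-keyed Inventory map and destroys the actor.
; Crafting functions check ingredient amounts, add crafted items from class defaults and decrement or remove stock.
; Amount-based removal probes four sides for a free point, but spawns nothing and ignores the result.
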(event `EnhancedInput|/Game/Input/Actions/IA_TakeItem`
  (params (ActionValue :type Boolean) (ElapsedSeconds :type "Float (double-precision)") (TriggeredSeconds :type "Float (double-precision)") (InputAction :type "InputAction Object Reference" :default "/Game/Input/Actions/IA_TakeItem.IA_TakeItem"))
  (bind _actorref (`self.ActorRef`))
  (bind _followcamera (`CelestiaSingsOfFateCharacter.FollowCamera` _actorref))
  (bind _returnvalue (`SceneComponent.K2_GetComponentLocation` _followcamera))
  (:`Completed`
    (bind _outhit (`KismetSystemLibrary.SphereTraceSingle` :`Start` _returnvalue :`End` (+ _returnvalue (* (`SceneComponent.GetForwardVector` _followcamera) (+ (`SpringArmComponent.TargetArmLength` (`CelestiaSingsOfFateCharacter.CameraBoom` _actorref)) 500.0))) :`Radius` 10.0 :`TraceChannel` "TraceTypeQuery1" :`DrawDebugType` "ForDuration"))
    (bind (_bblockinghit _binitialoverlap _time _distance _location _impactpoint _normal _impactnormal _physmat _hitactor) (`GameplayStatics.BreakHitResult` _outhit))
    (bind _added_ (`self.AddItem` _hitactor))
    (if _added_
      (`Actor.K2_DestroyActor` _hitactor))))

(fn `AddItem`
  (params (Actor :type "Actor Object Reference"))
  (returns (`Added?` :type Boolean))
  (locals (CurrentItem :type "/Game/Blueprints/Crafting/Objetos/S_PickupItem Structure"))
  (bind _currentitem (`local.CurrentItem`))
  (bind _asbp_base_pickup_item (cast `/Game/Blueprints/Crafting/Objetos/BP_BasePickupItem` Actor)
    (:`then`
      (bind _output_get (set `local.CurrentItem` (`/Game/Blueprints/Crafting/Objetos/BP_BasePickupItem.GetItemData` _asbp_base_pickup_item)))
      (if (`self.IsItemAlreadyInInventory` _output_get)
        (`self.IncrementAmount` _currentitem)
        (else
          (`self.AddItemToInventory` _currentitem)))
      (`KismetSystemLibrary.PrintString` (`KismetStringLibrary.Concat_StrStr` (`.Name_11_344F9DE44BADF61F8E9B0BB92CF84809` (break `/Game/Blueprints/Crafting/Objetos/S_PickupItem` _currentitem)) "Added"))
      (return true))
    (:`CastFailed`
      (set `local.CurrentItem` (struct))
      (return false))))

(fn `AddItemToInventory`
  (params (Item :type "/Game/Blueprints/Crafting/Objetos/S_PickupItem Structure"))
  (`BlueprintMapLibrary.Map_Add` (`self.Inventory`) (`.Name_11_344F9DE44BADF61F8E9B0BB92CF84809` (break `/Game/Blueprints/Crafting/Objetos/S_PickupItem` Item)) Item))

(fn `CanCraft`
  (params (Ingredients :type "Map of /Game/Blueprints/Crafting/Objetos/BP_BasePickupItem Soft Class Reference to Integer"))
  (returns (CanCraft :type Boolean))
  (bind _keys (`BlueprintMapLibrary.Map_Keys` Ingredients))
  (for _array_element _keys
    (bind (_value _returnvalue) (`BlueprintMapLibrary.Map_Find` (`self.Inventory`) (defaults `Object` (`|ConvertAsset` _array_element))))
    (if _returnvalue
      (if (not (>= (`.Amount_18_AD38B2EE4B89BD88D08D4A834B1D4FE8` (break `/Game/Blueprints/Crafting/Objetos/S_PickupItem` _value)) (`BlueprintMapLibrary.Map_Find` (`local.Ingredients`) _array_element)))
        (return false))
      (else
        (return false))))
  (return true))

(fn `CraftItme`
  (params (ClassItem :type "/Game/Blueprints/Crafting/Objetos/BP_BasePickupItem Soft Class Reference"))
  (bind (_name _description _category _value _id _amount _image) (defaults `Object` (`|ConvertAsset` ClassItem)))
  (bind _s_pickupitem (make `/Game/Blueprints/Crafting/Objetos/S_PickupItem` _name _value _description _category _id 1 _image))
  (bind (_itemdata _hasitem_) (`self.IsItemInInventory` _name))
  (if _hasitem_
    (`self.IncrementAmount` _s_pickupitem)
    (else
      (`self.AddItemToInventory` _s_pickupitem))))

(fn `GetItemAmountFromInventory`
  (params (ItemName :type String))
  (returns (Amount :type Integer))
  (return (`.Amount_18_AD38B2EE4B89BD88D08D4A834B1D4FE8` (break `/Game/Blueprints/Crafting/Objetos/S_PickupItem` (`BlueprintMapLibrary.Map_Find` (`self.Inventory`) ItemName)))))

(fn `GetStartEndTrace`
  (params (VectorDirection :type "Vector Structure"))
  (returns (Start :type "Vector Structure") (Ends :type "Vector Structure"))
  (bind _returnvalue (`SceneComponent.K2_GetComponentLocation` (`Character.Mesh` (`self.ActorRef`))))
  (return (+ _returnvalue (0.0 0.0 100.0)) (+ (+ _returnvalue VectorDirection) (0.0 0.0 100.0))))

(fn `IncrementAmount`
  (params (Item :type "/Game/Blueprints/Crafting/Objetos/S_PickupItem Structure"))
  (locals (ItemName :type String))
  (bind _value (`BlueprintMapLibrary.Map_Find` (`self.Inventory`) (`local.ItemName`)))
  (set `local.ItemName` (`.Name_11_344F9DE44BADF61F8E9B0BB92CF84809` (break `/Game/Blueprints/Crafting/Objetos/S_PickupItem` Item)))
  (bind _result (`/Engine/EditorBlueprintResources/StandardMacros.IncrementInt` (`.Amount_18_AD38B2EE4B89BD88D08D4A834B1D4FE8` (break `/Game/Blueprints/Crafting/Objetos/S_PickupItem` _value)))
    (:`  `
      (bind _structout (setmembers `/Game/Blueprints/Crafting/Objetos/S_PickupItem` :`StructRef` _value :`Amount` _result))
      (`BlueprintMapLibrary.Map_Add` (`self.Inventory`) (`local.ItemName`) _structout))))

(fn `IsItemAlreadyInInventory`
  (params (Items :type "/Game/Blueprints/Crafting/Objetos/S_PickupItem Structure"))
  (returns (ReturnValue :type Boolean))
  (return (`BlueprintMapLibrary.Map_Contains` (`self.Inventory`) (`.Name_11_344F9DE44BADF61F8E9B0BB92CF84809` (break `/Game/Blueprints/Crafting/Objetos/S_PickupItem` Items)))))

(fn `IsItemInInventory`
  (params (Name :type String))
  (returns (ItemData :type "/Game/Blueprints/Crafting/Objetos/S_PickupItem Structure") (`HasItem?` :type Boolean))
  (bind (_value _returnvalue) (`BlueprintMapLibrary.Map_Find` (`self.Inventory`) Name))
  (return _value _returnvalue))

(fn `RemoveIngredients`
  (params (RemoveIngredients :type "Map of /Game/Blueprints/Crafting/Objetos/BP_BasePickupItem Soft Class Reference to Integer") (SpawnItems :type Boolean))
  (bind _keys (`BlueprintMapLibrary.Map_Keys` RemoveIngredients))
  (for _array_element _keys
    (`self.RemoveItemByAmount` (defaults `Object` (`|ConvertAsset` _array_element)) (`BlueprintMapLibrary.Map_Find` RemoveIngredients _array_element) SpawnItems)))

(fn `RemoveItemByAmount`
  (params (Item :type String) (Amount :type Integer) (SpawnItems :type Boolean))
  (returns (UpdateItem :type "/Game/Blueprints/Crafting/Objetos/S_PickupItem Structure"))
  (locals (DeleteItem :type "/Game/Blueprints/Crafting/Objetos/S_PickupItem Structure") (DropAmount :type Integer) (FoundItem :type "/Game/Blueprints/Crafting/Objetos/S_PickupItem Structure"))
  (bind (_value _returnvalue) (`BlueprintMapLibrary.Map_Find` (`self.Inventory`) Item))
  (bind _value_2 (`BlueprintMapLibrary.Map_Find` (`self.Inventory`) (`local.Item`)))
  (if _returnvalue
    (set `local.FoundItem` _value)
    (for _ (range Amount)
      (bind _structout (setmembers `/Game/Blueprints/Crafting/Objetos/S_PickupItem` :`StructRef` (`local.FoundItem`) :`Amount` (- (`.Amount_18_AD38B2EE4B89BD88D08D4A834B1D4FE8` (break `/Game/Blueprints/Crafting/Objetos/S_PickupItem` _value)) 1)))
      (`BlueprintMapLibrary.Map_Add` (`self.Inventory`) (`local.Item`) _structout)
      (`self.TryTraceAround`))
    (if (== (`.Amount_18_AD38B2EE4B89BD88D08D4A834B1D4FE8` (break `/Game/Blueprints/Crafting/Objetos/S_PickupItem` _value_2)) 0)
      (`BlueprintMapLibrary.Map_Remove` (`self.Inventory`) (`local.Item`))
      (return)
      (else
        (return _value_2)))))

(fn `RemoveSingleItem`
  (params (Key :type "String (by ref)"))
  (returns (ItemFullRemoved :type Boolean) (NewItemData :type "/Game/Blueprints/Crafting/Objetos/S_PickupItem Structure"))
  (locals (DeletedItem :type "/Game/Blueprints/Crafting/Objetos/S_PickupItem Structure"))
  (bind (_value _returnvalue) (`BlueprintMapLibrary.Map_Find` (`self.Inventory`) Key))
  (bind ((`Amount_18_AD38B2EE4B89BD88D08D4A834B1D4FE8` _amount)) (break `/Game/Blueprints/Crafting/Objetos/S_PickupItem` _value))
  (if _returnvalue
    (if (>= _amount 1)
      (bind _structout (setmembers `/Game/Blueprints/Crafting/Objetos/S_PickupItem` :`StructRef` _value :`Amount` (- _amount 1)))
      (`BlueprintMapLibrary.Map_Add` (`self.Inventory`) (`local.Key`) _structout)
      (return false _structout)
      (else
        (set `local.DeletedItem` _value)
        (`BlueprintMapLibrary.Map_Remove` (`self.Inventory`) (`local.Key`))
        (return true)))))

(fn `TryTraceAround`
  (returns (Position :type "Vector Structure"))
  (bind (_start _ends) (`self.GetStartEndTrace` (* (`Actor.GetActorForwardVector` (`self.ActorRef`)) 100.0)))
  (bind (_outhit _returnvalue) (`KismetSystemLibrary.SphereTraceSingle` :`Start` _start :`End` _ends :`TraceChannel` "TraceTypeQuery1" :`DrawDebugType` "ForDuration"))
  (if _returnvalue
    (bind (_start_2 _ends_2) (`self.GetStartEndTrace` (* (`Actor.GetActorRightVector` (`self.ActorRef`)) 100.0)))
    (bind (_outhit_2 _returnvalue_2) (`KismetSystemLibrary.SphereTraceSingle` :`Start` _start_2 :`End` _ends_2 :`TraceChannel` "TraceTypeQuery1" :`DrawDebugType` "ForDuration"))
    (if _returnvalue_2
      (bind (_start_3 _ends_3) (`self.GetStartEndTrace` (* (`Actor.GetActorForwardVector` (`self.ActorRef`)) -100.0)))
      (bind (_outhit_3 _returnvalue_3) (`KismetSystemLibrary.SphereTraceSingle` :`Start` _start_3 :`End` _ends_3 :`TraceChannel` "TraceTypeQuery1" :`DrawDebugType` "ForDuration"))
      (if _returnvalue_3
        (bind (_start_4 _ends_4) (`self.GetStartEndTrace` (* (`Actor.GetActorRightVector` (`self.ActorRef`)) -100.0)))
        (bind (_outhit_4 _returnvalue_4) (`KismetSystemLibrary.SphereTraceSingle` :`Start` _start_4 :`End` _ends_4 :`TraceChannel` "TraceTypeQuery1" :`DrawDebugType` "ForDuration"))
        (if _returnvalue_4
          (bind (_bblockinghit _binitialoverlap _time _distance _location _impactpoint _normal _impactnormal _physmat _hitactor _hitcomponent _hitbonename _bonename _hititem _elementindex _faceindex _tracestart _traceend) (`GameplayStatics.BreakHitResult` _outhit_4))
          (return _impactpoint)
          (else
            (return _traceend)))
        (else
          (return (`.TraceEnd` (`GameplayStatics.BreakHitResult` _outhit_3)))))
      (else
        (return (`.TraceEnd` (`GameplayStatics.BreakHitResult` _outhit_2)))))
    (else
      (return (`.TraceEnd` (`GameplayStatics.BreakHitResult` _outhit))))))