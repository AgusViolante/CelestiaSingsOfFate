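; PC_Game is the game's player controller Blueprint, managing which Enhanced Input mapping contexts are active for the local player.
; On BeginPlay it adds the default, inventory, menu and mouse-look contexts, all at the same priority.
; RegisterContext and DeRegisterContext wrap the local player subsystem's add and remove calls so a given context can be switched on or off.
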(event `self.ReceiveBeginPlay`
  (bind _returnvalue (subsystem `EnhancedInputLocalPlayerSubsystem`))
  (`EnhancedInputSubsystemInterface.AddMappingContext` _returnvalue "/Game/Input/IMC_Default.IMC_Default" 0 (struct))
  (`EnhancedInputSubsystemInterface.AddMappingContext` _returnvalue "/Game/Input/IMC_InventoryControlls.IMC_InventoryControlls" 0 (struct))
  (`EnhancedInputSubsystemInterface.AddMappingContext` _returnvalue "/Game/Input/IMC_MenuControlls.IMC_MenuControlls" 0 (struct))
  (`EnhancedInputSubsystemInterface.AddMappingContext` _returnvalue "/Game/Input/IMC_MouseLook.IMC_MouseLook" 0 (struct)))

(fn `DeRegisterContext`
  (params (MappingContext :type "InputMappingContext Object Reference"))
  (`EnhancedInputSubsystemInterface.RemoveMappingContext` (subsystem `EnhancedInputLocalPlayerSubsystem`) MappingContext (struct)))

(fn `RegisterContext`
  (params (MappingContext :type "InputMappingContext Object Reference"))
  (`EnhancedInputSubsystemInterface.AddMappingContext` (subsystem `EnhancedInputLocalPlayerSubsystem`) MappingContext 0 (struct)))

(fn `UserConstructionScript`)